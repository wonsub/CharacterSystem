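; BP_SelectionCharacter is a selection character whose skeletal mesh switches between the entries of a Characters array.
; ChangeCharacter advances CharacterIndex, wraps to the first entry after the last, and applies that asset to the Mesh component.
; The event graph and construction script are empty, so the blueprint contains no call to ChangeCharacter.
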(fn `ChangeCharacter`
  (bind _returnvalue (+ (`self.CharacterIndex`) 1))
  (if (< _returnvalue (`KismetArrayLibrary.Array_Length` (`self.Characters`)))
    (bind _output_get (set `self.CharacterIndex` _returnvalue))
    (else
      (set `self.CharacterIndex` 0)))
  (`SkeletalMeshComponent.SetSkeletalMeshAsset` (`self.Mesh`) (`|GetArrayItem` (`self.Characters`) _output_get)))

(fn `UserConstructionScript`)