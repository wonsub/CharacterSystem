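; Player controller that lets the player cycle control between the third-person characters in the level with the Tab key.
; On BeginPlay it gathers every BP_ThirdPersonCharacter into a roster and records the player's character as the current one.
; Each Tab press calls NextCharacter, which finds the current character's index, advances it with wraparound to the first entry, then possesses that character.
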(event `self.ReceiveBeginPlay`
  (bind _outactors (`GameplayStatics.GetAllActorsOfClass` "/Game/ThirdPerson/Blueprints/BP_ThirdPersonCharacter.BP_ThirdPersonCharacter_C"))
  (set `self.CharacterRoaster` _outactors)
  (bind _asbp_third_person_character (cast `/Game/ThirdPerson/Blueprints/BP_ThirdPersonCharacter` (`GameplayStatics.GetPlayerCharacter` 0)))
  (set `self.CurrentCharacter` _asbp_third_person_character))

(event `Key|Tab`
  (params (Key :type "Key Structure"))
  (:`Pressed`
    (`self.NextCharacter`)))

(fn `NextCharacter`
  (locals (Local_Index :type Integer))
  (bind _returnvalue (`KismetArrayLibrary.Array_Find` (`self.CharacterRoaster`) (`self.CurrentCharacter`)))
  (bind _returnvalue_2 (+ _returnvalue 1))
  (set `local.Local_Index` _returnvalue)
  (bind _output_get (set `local.Local_Index` (`KismetMathLibrary.SelectInt` _returnvalue_2 0 (`KismetArrayLibrary.Array_IsValidIndex` (`self.CharacterRoaster`) _returnvalue_2))))
  (bind _output_get_2 (set `self.CurrentCharacter` (`|GetArrayItem` (`self.CharacterRoaster`) _output_get)))
  (`self.Possess` _output_get_2))

(fn `UserConstructionScript`)